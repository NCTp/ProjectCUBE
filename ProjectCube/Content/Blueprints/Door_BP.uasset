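; Door_BP is a holographic door whose IsLocked flag decides whether it blocks or lets things through.
; When locked, the mesh uses one holo-refract material and both mesh and box have query and physics collision; when unlocked, it swaps material and disables both collisions.
; The construction script applies this state in the editor, and Tick reapplies the same duplicated logic every frame rather than reacting to changes.
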(event EventTick
  (params (DeltaSeconds :type Float%20%28single-precision%29))
  (bind _mesh (Variables|Default|GetMesh))
  (bind _mesh_2 (Variables|Default|GetMesh))
  (bind _box (Variables|Default|GetBox))
  (if (Variables|Default|GetIsLocked)
    (Rendering|Material|SetMaterial _mesh 0 "/Game/SuperGrid/StarterPack/Materials/Base/M_SuperGrid_HoloRefract_2.M_SuperGrid_HoloRefract_2")
    (Collision|SetCollisionEnabled _mesh_2 "QueryAndPhysics")
    (Collision|SetCollisionEnabled _box "QueryAndPhysics")
    (else
      (Rendering|Material|SetMaterial _mesh 0 "/Game/SuperGrid/StarterPack/Materials/Base/M_SuperGrid_HoloRefract.M_SuperGrid_HoloRefract")
      (Collision|SetCollisionEnabled _mesh_2 "NoCollision")
      (Collision|SetCollisionEnabled _box "NoCollision"))))

(fn ConstructionScript
  (bind _mesh (Variables|Default|GetMesh))
  (bind _mesh_2 (Variables|Default|GetMesh))
  (bind _box (Variables|Default|GetBox))
  (if (Variables|Default|GetIsLocked)
    (Rendering|Material|SetMaterial _mesh 0 "/Game/SuperGrid/StarterPack/Materials/Base/M_SuperGrid_HoloRefract_2.M_SuperGrid_HoloRefract_2")
    (Collision|SetCollisionEnabled _mesh_2 "QueryAndPhysics")
    (Collision|SetCollisionEnabled _box "QueryAndPhysics")
    (else
      (Rendering|Material|SetMaterial _mesh 0 "/Game/SuperGrid/StarterPack/Materials/Base/M_SuperGrid_HoloRefract.M_SuperGrid_HoloRefract")
      (Collision|SetCollisionEnabled _mesh_2 "NoCollision")
      (Collision|SetCollisionEnabled _box "NoCollision"))))