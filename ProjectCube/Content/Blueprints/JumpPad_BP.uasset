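; JumpPad_BP is a configurable pad for the FirstPersonCharacter that acts as a jump pad or acceleration pad, and can move.
; Box overlap either launches the character upward by scaled jump velocity or sets a new walk speed with zero friction and braking.
; Ending actor overlap restores hardcoded movement values for acceleration pads.
; When IsMoving, a timeline moves the mesh, with a Delay on its Update toggling Loop to alternate play and reverse.
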(event OnComponentBeginOverlap(Box)
  (params (OverlappedComponent :type Primitive%20Component%20Object%20Reference) (OtherActor :type Actor%20Object%20Reference) (OtherComp :type Primitive%20Component%20Object%20Reference) (OtherBodyIndex :type Integer) (bFromSweep :type Boolean) (SweepResult :type Hit%20Result%20Structure%20%28by%20ref%29))
  (bind _asfirst_person_character (Utilities|Casting|CastToFirstPersonCharacter OtherActor))
  (if (Variables|Default|GetIsJumpPad)
    (Character|LaunchCharacter _asfirst_person_character (Math|Vector|MakeVector 0.0 0.0 (* (Variables|/Script/Engine.CharacterMovementComponent|GetJumpZVelocity (Variables|/Script/Engine.Character|GetCharacterMovement _asfirst_person_character)) (Variables|Default|GetJumpPower))) false true)
    (elif (Variables|Default|GetIsAccelPad)
      (Variables|/Script/Engine.CharacterMovementComponent|SetMaxWalkSpeed (Variables|/Script/Engine.Character|GetCharacterMovement _asfirst_person_character) (Variables|Default|GetWalkSpeed))
      (Variables|/Script/Engine.CharacterMovementComponent|SetGroundFriction (Variables|/Script/Engine.Character|GetCharacterMovement _asfirst_person_character) 0.0)
      (Variables|/Script/Engine.CharacterMovementComponent|SetBrakingDecelerationWalking (Variables|/Script/Engine.Character|GetCharacterMovement _asfirst_person_character) 0.0))))

(event EventBeginPlay
  (if (Variables|Default|GetIsMoving)
    (bind _newtrack_0 (Timeline|Moving Play)
      (:Update
        (Transformation|SetRelativeLocation (Variables|Default|GetStaticMesh) _newtrack_0 false false)
        (Utilities|FlowControl|Delay 3.0)
        (if (Variables|Default|GetLoop)
          (Variables|Default|SetLoop false)
          (Timeline|Moving Reverse)
          (else
            (Variables|Default|SetLoop true)
            (Timeline|Moving Play)))))))

(event Collision|EventActorEndOverlap
  (params (OtherActor :type Actor%20Object%20Reference))
  (bind _asfirst_person_character (Utilities|Casting|CastToFirstPersonCharacter OtherActor))
  (if (Variables|Default|GetIsAccelPad)
    (Variables|/Script/Engine.CharacterMovementComponent|SetMaxWalkSpeed (Variables|/Script/Engine.Character|GetCharacterMovement _asfirst_person_character) 8e+02)
    (Variables|/Script/Engine.CharacterMovementComponent|SetGroundFriction (Variables|/Script/Engine.Character|GetCharacterMovement _asfirst_person_character) 8.0)
    (Variables|/Script/Engine.CharacterMovementComponent|SetBrakingDecelerationWalking (Variables|/Script/Engine.Character|GetCharacterMovement _asfirst_person_character) 2048.0)))

(fn ConstructionScript)